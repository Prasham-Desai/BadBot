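; BP_BlasterBeam is a blaster projectile that damages whatever it hits, then destroys itself.
; When BeamMesh registers a hit, HandlePawnHit spawns the NS_BeamBurst effect at the impact point, oriented along the hit normal, and checks whether the actor implements BPI_Damageable.
; Damageable actors receive BeamDamage through GetHurtMessage, and the beam destroys itself on any hit.
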(event OnComponentHit(BeamMesh)
  (params (HitComponent :type Primitive%20Component%20Object%20Reference) (OtherActor :type Actor%20Object%20Reference) (OtherComp :type Primitive%20Component%20Object%20Reference) (NormalImpulse :type Vector :default "0, 0, 0") (Hit :type Hit%20Result%20Structure%20%28by%20ref%29))
  (bind _output_get (Variables|Default|SetHItActor OtherActor))
  (bind _returnvalue (CallFunction|HandlePawnHit _output_get Hit))
  (if _returnvalue
    (Class|BPIDamageable|GetHurt(Message) (Variables|Default|GetHItActor) (Variables|Default|GetBeamDamage)))
  (Actor|DestroyActor))

(fn ConstructionScript)

(fn HandlePawnHit
  (params (Hit%20Actor :type Object%20Object%20Reference) (Hit%20Result :type Hit%20Result%20Structure%20%28by%20ref%29))
  (bind (_bblockinghit _binitialoverlap _time _distance _location _impactpoint _normal) (Collision|BreakHitResult Hit%20Result))
  (Niagara|SpawnSystematLocation "/Game/FX/NS_BeamBurst.NS_BeamBurst" _impactpoint (Math|Rotator|MakeRotfromX _normal))
  (return (Utilities|DoesObjectImplementInterface Hit%20Actor "/Game/Blueprints/Interfaces/BPI_Damageable.BPI_Damageable_C")))