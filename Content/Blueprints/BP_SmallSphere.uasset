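; BP_SmallSphere is a moving, spinning collectible that raises the score in BP_BadBotGameMode when a Pawn overlaps it.
; On BeginPlay it scales in via a timeline, picks a random spin and starts a lifetime timer.
; Tick moves it along its forward vector and applies the spin.
; Pickup or timeout triggers WinkOut, guarded against repeats, which scales the mesh by timeline and then destroys the actor.
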(event OnComponentBeginOverlap(SphereVolume)
  (params (OverlappedComponent :type Primitive%20Component%20Object%20Reference) (OtherActor :type Actor%20Object%20Reference) (OtherComp :type Primitive%20Component%20Object%20Reference) (OtherBodyIndex :type Integer) (bFromSweep :type Boolean) (SweepResult :type Hit%20Result%20Structure%20%28by%20ref%29))
  ;[0 0.15 0.1446 0.5] Collision Detection
  (if (Class|GameplayStatics|ObjectIsA OtherActor "/Script/Engine.Pawn")
    (bind _asbp_bad_bot_game_mode (Utilities|Casting|CastToBP_BadBotGameMode (Game|GetGameMode)))
    (Default|IncrementScore _asbp_bad_bot_game_mode)
    (CallFunction|WinkOut)))

(event Custom|WinkOut
  ;[0.15 0 0.08854 0.5] Random Rotation
  (if (not (Variables|Default|GetIsWinking))
    (Variables|Default|SetIsWinking true)
    (bind _scale (Timeline|WinkOutTimeline Play)
      (:Update
        (CallFunction|ScaleDownSphere _scale))
      (:Finished
        (Actor|DestroyActor)))))

(event Custom|WinkIn
  ;[0 0.06624 0.15 0.5] WinkIn to Exsiting
  (bind _scale (Timeline|WinkIn%20Timeline Play)
    (:Update
      (Transformation|SetWorldScale3D (Variables|Default|GetSmallSphereMesh) _scale))))

(event EventBeginPlay
  ;[0.15 0 0.08854 0.5] Random Rotation
  (CallFunction|Winkin)
  (CallFunction|InitDeltaRotation)
  (Utilities|Time|SetTimerbyEvent (delegate Custom|WinkOut) (Variables|SphereMovement|GetSmallSphereLifeTime)))

(event EventTick
  (params (DeltaSeconds :type Float%20%28single-precision%29))
  ;[0.03351 0.15 0 0.5] Sphere Movement
  (CallFunction|UpdateLocation DeltaSeconds)
  (CallFunction|UpdateRotation DeltaSeconds))

(fn ConstructionScript)

(fn UpdateLocation
  (params (Delta%20Seconds :type Float%20%28double-precision%29))
  (Transformation|AddActorWorldOffset (* (* Delta%20Seconds (Variables|SphereMovement|GetSmallSphereSpeed)) (Transformation|GetActorForwardVector)))
  (return))

(fn InitDeltaRotation
  (Variables|SphereMovement|SetSmallSphereRotator (* (Math|Random|RandomRotator false) (Variables|SphereMovement|GetRotationScaleFactor))))

(fn UpdateRotation
  (params (Delta%20Speed :type Float%20%28single-precision%29))
  (Class|Actor|AddActorWorldRotation (* (Variables|SphereMovement|GetSmallSphereRotator) Delta%20Speed)))

(fn ScaleDownSphere
  (params (Scale :type Float%20%28double-precision%29))
  (Transformation|SetWorldScale3D (Variables|Default|GetSmallSphereMesh) (Math|Conversions|ToVector(Float) Scale)))