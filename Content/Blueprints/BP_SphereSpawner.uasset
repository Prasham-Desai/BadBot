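; BP_SphereSpawner is an actor that periodically spawns BP_SmallSphere actors at random points around itself.
; BeginPlay starts a looping timer that calls the function named by SpawnFunctionName every SpawnTime seconds.
; SpawnSmallSphere places each sphere with random yaw at a point from GetRandomPointInSphere.
; That point uses a random direction and a linearly random distance up to SpawnRadius, so spawns cluster toward the center.
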(event EventBeginPlay
  ;[0.15 0.1167 0 0.5] Start Sphere Spawn Timer
  (Utilities|Time|SetTimerbyFunctionName 0 (Variables|SphereSpawner|GetSpawnFunctionName) (Variables|SphereSpawner|GetSpawnTime) true))

(fn ConstructionScript)

(fn GetRandomPointinSphere
  (return (+ (* (Math|Vector|GetForwardVector (Math|Random|RandomRotator false)) (Math|Random|RandomFloatinRange 0.0 (Variables|SphereSpawner|GetSpawnRadius))) (Transformation|GetActorLocation))))

(fn SpawnSmallSphere
  (Game|SpawnActorfromClass "/Game/Blueprints/BP_SmallSphere.BP_SmallSphere_C" (Math|Transform|MakeTransform (CallFunction|GetRandomPointinSphere) (Math|Rotator|MakeRotator 0.0 0.0 (.yaw (Math|Random|RandomRotator false))) "1.000000,1.000000,1.000000") "Undefined" "MultiplyWithRoot" 0 0))